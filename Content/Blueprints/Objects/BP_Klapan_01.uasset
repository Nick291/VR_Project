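; BP_Klapan_01 is an interactable object, by its name a valve, that can be attached to a given component and released.
; Interact toggles on IsAtach: it either turns off Cube physics and snaps to the AtachTo component's location and rotation, or detaches in world space and re-enables physics.
; The construction script gives Cube a dynamic material instance tinted magenta.
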(event EventInteract
  (params (AtachTo :type Scene%20Component%20Object%20Reference))
  (if (Variables|Default|GetIsAtach?)
    (Transformation|DetachFromActor "KeepWorld" "KeepWorld" "KeepWorld")
    (Physics|SetSimulatePhysics (Variables|Default|GetCube) true)
    (Variables|Default|SetIsAtach? false)
    (else
      (Physics|SetSimulatePhysics (Variables|Default|GetCube) false)
      (Transformation|AttachComponentToComponent AtachTo "None" "SnapToTarget" "SnapToTarget" "KeepWorld" false)
      (Variables|Default|SetIsAtach? true))))

(fn ConstructionScript
  (bind _returnvalue (Rendering|Material|CreateDynamicMaterialInstance (Variables|Default|GetCube) 0 0 "None" :!class /Script/Engine.PrimitiveComponent))
  (Rendering|Material|SetVectorParameterValue _returnvalue "Color" "(R=1.000000,G=0.000000,B=1.000000,A=1.000000)" :!class /Script/Engine.MaterialInstanceDynamic))