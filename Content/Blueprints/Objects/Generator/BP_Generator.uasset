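; Generator puzzle actor whose button toggles the first BP_Light found, but only while both a "Bachok" and a "Radiator" part are inserted.
; Tagged parts entering their trigger receive InteractMessage with the slot's ghost component and release the player's hold; removing either switches the light off.
; Ghost meshes preview empty slots on proximity.
; Button overlap enables input and shows a prompt yawed toward the player every Tick; an incomplete generator's button just bounces back.
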(event OnComponentBeginOverlap(Bottom_Collision)
  (params (OverlappedComponent :type Primitive%20Component%20Object%20Reference) (OtherActor :type Actor%20Object%20Reference) (OtherComp :type Primitive%20Component%20Object%20Reference) (OtherBodyIndex :type Integer) (bFromSweep :type Boolean) (SweepResult :type Hit%20Result%20Structure%20%28by%20ref%29))
  ;[1 1 1] Button
  (Input|EnableInput (Game|GetPlayerController 0))
  (Rendering|SetVisibility (Variables|Default|GetPress_Bottom) true false))

(event OnComponentEndOverlap(Bottom_Collision)
  (params (OverlappedComponent :type Primitive%20Component%20Object%20Reference) (OtherActor :type Actor%20Object%20Reference) (OtherComp :type Primitive%20Component%20Object%20Reference) (OtherBodyIndex :type Integer))
  ;[1 1 1] Button
  (Input|DisableInput (Game|GetPlayerController 0))
  (Rendering|SetVisibility (Variables|Default|GetPress_Bottom) false false))

(event OnComponentBeginOverlap(Rox)
  (params (OverlappedComponent :type Primitive%20Component%20Object%20Reference) (OtherActor :type Actor%20Object%20Reference) (OtherComp :type Primitive%20Component%20Object%20Reference) (OtherBodyIndex :type Integer) (bFromSweep :type Boolean) (SweepResult :type Hit%20Result%20Structure%20%28by%20ref%29))
  (Utilities|FlowControl|Sequence
    (:then_0
      (if (not (Variables|Default|GetBachokIsActiv?))
        (Rendering|SetVisibility (Variables|Default|GetGhost_Bachok) true false)))
    (:then_1
      (if (not (Variables|Default|GetRadiatorIsActiv?))
        (Rendering|SetVisibility (Variables|Default|GetGhost_Radiator) true false)))))

(event OnComponentEndOverlap(Rox)
  (params (OverlappedComponent :type Primitive%20Component%20Object%20Reference) (OtherActor :type Actor%20Object%20Reference) (OtherComp :type Primitive%20Component%20Object%20Reference) (OtherBodyIndex :type Integer))
  (Utilities|FlowControl|Sequence
    (:then_0
      (if (not (Variables|Default|GetBachokIsActiv?))
        (Rendering|SetVisibility (Variables|Default|GetGhost_Bachok) false false)))
    (:then_1
      (if (not (Variables|Default|GetRadiatorIsActiv?))
        (Rendering|SetVisibility (Variables|Default|GetGhost_Radiator) false false)))))

(event OnComponentBeginOverlap(Capsule)
  (params (OverlappedComponent :type Primitive%20Component%20Object%20Reference) (OtherActor :type Actor%20Object%20Reference) (OtherComp :type Primitive%20Component%20Object%20Reference) (OtherBodyIndex :type Integer) (bFromSweep :type Boolean) (SweepResult :type Hit%20Result%20Structure%20%28by%20ref%29))
  (if (Components|ComponentHasTag (Variables|/Script/Engine.Actor|GetRootComponent OtherActor) "Bachok")
    (Class|BPIInteractible|Interact(Message) OtherActor (Variables|Default|GetGhost_Bachok))
    (bind _asfirst_person_character (Utilities|Casting|CastToFirstPersonCharacter (Game|GetPlayerCharacter 0)))
    (Variables|/Game/FirstPersonBP/Blueprints/FirstPersonCharacter.FirstPersonCharacter_C|SetIsHoldingObject _asfirst_person_character false)
    (Rendering|SetVisibility (Variables|Default|GetGhost_Bachok) false false)
    (Variables|Default|SetBachokIsActiv? true)
    (Development|PrintString "Bachok In")))

(event OnComponentBeginOverlap(Box)
  (params (OverlappedComponent :type Primitive%20Component%20Object%20Reference) (OtherActor :type Actor%20Object%20Reference) (OtherComp :type Primitive%20Component%20Object%20Reference) (OtherBodyIndex :type Integer) (bFromSweep :type Boolean) (SweepResult :type Hit%20Result%20Structure%20%28by%20ref%29))
  (if (Components|ComponentHasTag (Variables|/Script/Engine.Actor|GetRootComponent OtherActor) "Radiator")
    (Class|BPIInteractible|Interact(Message) OtherActor (Variables|Default|GetGhost_Radiator))
    (bind _asfirst_person_character (Utilities|Casting|CastToFirstPersonCharacter (Game|GetPlayerCharacter 0)))
    (Variables|/Game/FirstPersonBP/Blueprints/FirstPersonCharacter.FirstPersonCharacter_C|SetIsHoldingObject _asfirst_person_character false)
    (Rendering|SetVisibility (Variables|Default|GetGhost_Radiator) false false)
    (Variables|Default|SetRadiatorIsActiv? true)
    (Development|PrintString "Radiator In")))

(event OnComponentEndOverlap(Capsule)
  (params (OverlappedComponent :type Primitive%20Component%20Object%20Reference) (OtherActor :type Actor%20Object%20Reference) (OtherComp :type Primitive%20Component%20Object%20Reference) (OtherBodyIndex :type Integer))
  (if (Components|ComponentHasTag (Variables|/Script/Engine.Actor|GetRootComponent OtherActor) "Bachok")
    (Class|BPIInteractible|Interact(Message) OtherActor (Variables|Default|GetGhost_Bachok))
    (Rendering|SetVisibility (Variables|Default|GetGhost_Bachok) true false)
    (Variables|Default|SetBachokIsActiv? false)
    (Development|PrintString "Bachok Out")
    (if (Variables|Default|GetIsLightOn?)
      (Transformation|AddLocalOffset (Variables|Default|GetBottom) "0, 0,5.000000" false false)
      (bind _outactors (Actor|GetAllActorsOfClass "/Game/Blueprints/Objects/Generator/BP_Light.BP_Light_C"))
      (Rendering|SetVisibility (Variables|/Game/Blueprints/Objects/Generator/BP_Light.BP_Light_C|GetPointLight (Utilities|Array|Get(acopy) _outactors)) false false)
      (Variables|Default|SetIsLightOn? false))))

(event OnComponentEndOverlap(Box)
  (params (OverlappedComponent :type Primitive%20Component%20Object%20Reference) (OtherActor :type Actor%20Object%20Reference) (OtherComp :type Primitive%20Component%20Object%20Reference) (OtherBodyIndex :type Integer))
  (if (Components|ComponentHasTag (Variables|/Script/Engine.Actor|GetRootComponent OtherActor) "Radiator")
    (Class|BPIInteractible|Interact(Message) OtherActor (Variables|Default|GetGhost_Radiator))
    (Rendering|SetVisibility (Variables|Default|GetGhost_Radiator) true false)
    (Variables|Default|SetRadiatorIsActiv? false)
    (Development|PrintString "Radiator Out")
    (if (Variables|Default|GetIsLightOn?)
      (Transformation|AddLocalOffset (Variables|Default|GetBottom) "0, 0,5.000000" false false)
      (bind _outactors (Actor|GetAllActorsOfClass "/Game/Blueprints/Objects/Generator/BP_Light.BP_Light_C"))
      (Rendering|SetVisibility (Variables|/Game/Blueprints/Objects/Generator/BP_Light.BP_Light_C|GetPointLight (Utilities|Array|Get(acopy) _outactors)) false false)
      (Variables|Default|SetIsLightOn? false))))

(event EventBeginPlay)

(event Collision|EventActorBeginOverlap
  (params (OtherActor :type Actor%20Object%20Reference)))

(event EventTick
  (params (DeltaSeconds :type Float%20%28single-precision%29))
  (CallFunction|GetRotation))

(event Input|ActionEvents|InputActionAction_Buttom
  (params (Key :type Key%20Structure))
  (bind _bachokisactiv_ (Variables|Default|GetBachokIsActiv?))
  (bind _radiatorisactiv_ (Variables|Default|GetRadiatorIsActiv?))
  (bind _bottom (Variables|Default|GetBottom))
  (bind _bottom_2 (Variables|Default|GetBottom))
  (bind _returnvalue (and _bachokisactiv_ _radiatorisactiv_))
  ;[1 1 1] Button
  (:Pressed
    (if (and (Variables|Default|GetBachokIsActiv?) (Variables|Default|GetRadiatorIsActiv?))
      (if (Variables|Default|GetIsLightOn?)
        (Transformation|AddLocalOffset _bottom_2 "0, 0,5.000000" false false)
        (if _returnvalue
          (bind _outactors (Actor|GetAllActorsOfClass "/Game/Blueprints/Objects/Generator/BP_Light.BP_Light_C"))
          (Rendering|SetVisibility (Variables|/Game/Blueprints/Objects/Generator/BP_Light.BP_Light_C|GetPointLight (Utilities|Array|Get(acopy) _outactors)) false false)
          (Variables|Default|SetIsLightOn? false))
        (else
          (Transformation|AddLocalOffset _bottom_2 "0, 0,-5.000000" false false)
          (if _returnvalue
            (bind _outactors_2 (Actor|GetAllActorsOfClass "/Game/Blueprints/Objects/Generator/BP_Light.BP_Light_C"))
            (Rendering|SetVisibility (Variables|/Game/Blueprints/Objects/Generator/BP_Light.BP_Light_C|GetPointLight (Utilities|Array|Get(acopy) _outactors_2)) true false)
            (Variables|Default|SetIsLightOn? true))))
      (elif (not (Variables|Default|GetIsBottomOn?))
        (Transformation|AddLocalOffset _bottom "0, 0,-5.000000" false false)
        (Variables|Default|SetIsBottomOn? true)
        (Utilities|FlowControl|Delay 0.25)
        (Transformation|AddLocalOffset _bottom "0, 0,5.000000" false false)
        (Variables|Default|SetIsBottomOn? false)))))

(fn ConstructionScript)

(fn GetRotation
  (bind _outactors (Actor|GetAllActorsOfClass "/Game/FirstPersonBP/Blueprints/FirstPersonCharacter.FirstPersonCharacter_C"))
  (Transformation|SetRelativeRotation (Variables|Default|GetPress_Bottom) (Math|Rotator|MakeRotator 0.0 0.0 (.yaw (Math|Rotator|FindLookatRotation (Transformation|GetWorldLocation (Variables|Default|GetPress_Bottom)) (Transformation|GetActorLocation (Utilities|Array|Get(acopy) _outactors))))) false false))