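; BP_Bachok is an interactable object that can be attached to a supplied component and detached again.
; Interact toggles on IsAtach, either disabling Bachok's physics and snapping to the AtachTo component, or detaching while keeping world transform.
; The detach branch does not turn physics simulation back on.
; Sphere overlap events are empty, and player input enable/disable calls are left unconnected.
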(event OnComponentBeginOverlap(Sphere)
  (params (OverlappedComponent :type Primitive%20Component%20Object%20Reference) (OtherActor :type Actor%20Object%20Reference) (OtherComp :type Primitive%20Component%20Object%20Reference) (OtherBodyIndex :type Integer) (bFromSweep :type Boolean) (SweepResult :type Hit%20Result%20Structure%20%28by%20ref%29)))

(event OnComponentEndOverlap(Sphere)
  (params (OverlappedComponent :type Primitive%20Component%20Object%20Reference) (OtherActor :type Actor%20Object%20Reference) (OtherComp :type Primitive%20Component%20Object%20Reference) (OtherBodyIndex :type Integer)))

(event EventInteract
  (params (AtachTo :type Scene%20Component%20Object%20Reference))
  (if (Variables|Default|GetIsAtach?)
    (Transformation|DetachFromActor "KeepWorld" "KeepWorld" "KeepWorld")
    (Variables|Default|SetIsAtach? false)
    (else
      (Physics|SetSimulatePhysics (Variables|Default|GetBachok) false)
      (Transformation|AttachComponentToComponent AtachTo "None" "SnapToTarget" "SnapToTarget" "KeepWorld" false)
      (Variables|Default|SetIsAtach? true))))

(event Input|ActionEvents|InputActionAction_Buttom
  (params (Key :type Key%20Structure :default "None")))

(fn ConstructionScript)