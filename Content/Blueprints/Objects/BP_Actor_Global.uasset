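; BP_Actor_Global is an assembly station where the player slots a sphere, then a cube, guided by ghost previews.
; Box_Coll shows the next missing piece's ghost.
; Tagged overlaps on Sphere and Box send InteractMessage with an attach target, track attach flags and clear the player's holding state on entry.
; The cube requires an attached sphere, and removing the sphere also messages the first BP_Cube_Actor_01 found.
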(event OnComponentEndOverlap(Sphere)
  (params (OverlappedComponent :type Primitive%20Component%20Object%20Reference) (OtherActor :type Actor%20Object%20Reference) (OtherComp :type Primitive%20Component%20Object%20Reference) (OtherBodyIndex :type Integer))
  ;[1 1 1] Attach Sphere
  (if (Components|ComponentHasTag (Variables|/Script/Engine.Actor|GetRootComponent OtherActor) "Sphere_Actor")
    (Class|BPIInteractible|Interact(Message) OtherActor (Variables|Default|GetScene))
    (Rendering|SetVisibility (Variables|Default|GetGhost_Spher) true false)
    (Variables|Default|SetSpherIsAttach? false)
    (Rendering|SetVisibility (Variables|Default|GetGhost_Cube) false false)
    (bind _outactors (Actor|GetAllActorsOfClass "/Game/Blueprints/Objects/BP_Cube_Actor_01.BP_Cube_Actor_01_C"))
    (Class|BPIInteractible|Interact(Message) (Utilities|Array|Get(acopy) _outactors))
    (Development|PrintString "Spher Out")))

(event OnComponentBeginOverlap(Sphere)
  (params (OverlappedComponent :type Primitive%20Component%20Object%20Reference) (OtherActor :type Actor%20Object%20Reference) (OtherComp :type Primitive%20Component%20Object%20Reference) (OtherBodyIndex :type Integer) (bFromSweep :type Boolean) (SweepResult :type Hit%20Result%20Structure%20%28by%20ref%29))
  ;[1 1 1] Attach Sphere
  (if (Components|ComponentHasTag (Variables|/Script/Engine.Actor|GetRootComponent OtherActor) "Sphere_Actor")
    (Class|BPIInteractible|Interact(Message) OtherActor (Variables|Default|GetScene))
    (bind _asfirst_person_character (Utilities|Casting|CastToFirstPersonCharacter (Game|GetPlayerCharacter 0)))
    (Variables|/Game/FirstPersonBP/Blueprints/FirstPersonCharacter.FirstPersonCharacter_C|SetIsHoldingObject _asfirst_person_character false)
    (Rendering|SetVisibility (Variables|Default|GetGhost_Spher) false false)
    (Variables|Default|SetSpherIsAttach? true)
    (Rendering|SetVisibility (Variables|Default|GetGhost_Cube) true false)
    (Development|PrintString "Spher In")))

(event OnComponentEndOverlap(Box_Coll)
  (params (OverlappedComponent :type Primitive%20Component%20Object%20Reference) (OtherActor :type Actor%20Object%20Reference) (OtherComp :type Primitive%20Component%20Object%20Reference) (OtherBodyIndex :type Integer))
  (Rendering|SetVisibility (Variables|Default|GetGhost_Spher) false false)
  (Rendering|SetVisibility (Variables|Default|GetGhost_Cube) false false))

(event OnComponentBeginOverlap(Box_Coll)
  (params (OverlappedComponent :type Primitive%20Component%20Object%20Reference) (OtherActor :type Actor%20Object%20Reference) (OtherComp :type Primitive%20Component%20Object%20Reference) (OtherBodyIndex :type Integer) (bFromSweep :type Boolean) (SweepResult :type Hit%20Result%20Structure%20%28by%20ref%29))
  (if (Variables|Default|GetSpherIsAttach?)
    (if (not (Variables|Default|GetCubeIsAttach?))
      (Rendering|SetVisibility (Variables|Default|GetGhost_Cube) true false))
    (else
      (Rendering|SetVisibility (Variables|Default|GetGhost_Spher) true false))))

(event OnComponentBeginOverlap(Box)
  (params (OverlappedComponent :type Primitive%20Component%20Object%20Reference) (OtherActor :type Actor%20Object%20Reference) (OtherComp :type Primitive%20Component%20Object%20Reference) (OtherBodyIndex :type Integer) (bFromSweep :type Boolean) (SweepResult :type Hit%20Result%20Structure%20%28by%20ref%29))
  (if (Components|ComponentHasTag (Variables|/Script/Engine.Actor|GetRootComponent OtherActor) "Cube_Actor")
    (if (Variables|Default|GetSpherIsAttach?)
      (Class|BPIInteractible|Interact(Message) OtherActor (Variables|Default|GetGhost_Cube))
      (bind _asfirst_person_character (Utilities|Casting|CastToFirstPersonCharacter (Game|GetPlayerCharacter 0)))
      (Variables|/Game/FirstPersonBP/Blueprints/FirstPersonCharacter.FirstPersonCharacter_C|SetIsHoldingObject _asfirst_person_character false)
      (Rendering|SetVisibility (Variables|Default|GetGhost_Cube) false false)
      (Variables|Default|SetCubeIsAttach? true)
      (Development|PrintString "Cube In"))))

(event OnComponentEndOverlap(Box)
  (params (OverlappedComponent :type Primitive%20Component%20Object%20Reference) (OtherActor :type Actor%20Object%20Reference) (OtherComp :type Primitive%20Component%20Object%20Reference) (OtherBodyIndex :type Integer))
  (if (Components|ComponentHasTag (Variables|/Script/Engine.Actor|GetRootComponent OtherActor) "Cube_Actor")
    (if (Variables|Default|GetSpherIsAttach?)
      (Class|BPIInteractible|Interact(Message) OtherActor (Variables|Default|GetGhost_Cube))
      (Rendering|SetVisibility (Variables|Default|GetGhost_Cube) true false)
      (Variables|Default|SetCubeIsAttach? false)
      (Development|PrintString "Cube Out"))))

(fn ConstructionScript)