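; BP_Tube_Klapp is an interactable physics prop that toggles between being attached and being loose.
; Its Interact event checks IsAtach: when free, it turns off mesh physics and snaps onto the passed AtachTo component, keeping world scale.
; When attached, it detaches in place and re-enables physics.
; The construction script does nothing, and a dynamic material creation node is left unconnected.
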(event EventInteract
  (params (AtachTo :type Scene%20Component%20Object%20Reference))
  (if (Variables|Default|GetIsAtach?)
    (Transformation|DetachFromActor "KeepWorld" "KeepWorld" "KeepWorld")
    (Physics|SetSimulatePhysics (Variables|Default|GetStaticMesh) true)
    (Variables|Default|SetIsAtach? false)
    (else
      (Physics|SetSimulatePhysics (Variables|Default|GetStaticMesh) false)
      (Transformation|AttachComponentToComponent AtachTo "None" "SnapToTarget" "SnapToTarget" "KeepWorld" false)
      (Variables|Default|SetIsAtach? true))))

(fn ConstructionScript)