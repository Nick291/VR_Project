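; BP_Collector_01_1 is a physics-driven collector part that toggles between attached and loose through its Attaching event.
; When attached, the event detaches the actor in place and turns physics simulation back on.
; When loose, it disables physics and a timeline lerps the mesh toward the target component's location and rotation.
; A one-second delay started from the timeline update then snap-attaches it, sets the attached flag and resets the timeline time.
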(event EventAttaching
  (params (Attach_To :type Scene%20Component%20Object%20Reference))
  (bind _sm_collector_01 (Variables|Default|GetSM_Collector_01))
  (if (Variables|Default|GetIsAtach?)
    (Transformation|DetachFromActor "KeepWorld" "KeepWorld" "KeepWorld")
    (Physics|SetSimulatePhysics (Variables|Default|GetSM_Collector_01) true)
    (Variables|Default|SetIsAtach? false)
    (else
      (Physics|SetSimulatePhysics (Variables|Default|GetSM_Collector_01) false)
      (bind _newtrack_0 (Timeline|Timeline_0 Play)
        (:Update
          (if (not (Variables|Default|GetIsAtach?))
            (Transformation|SetWorldTransform (Variables|Default|GetSM_Collector_01) (Math|Transform|MakeTransform (Math|Vector|Lerp(Vector) (Transformation|GetWorldLocation _sm_collector_01) (Transformation|GetWorldLocation Attach_To) _newtrack_0) (Math|Rotator|Lerp(Rotator) (Transformation|GetWorldRotation _sm_collector_01) (Transformation|GetWorldRotation Attach_To) _newtrack_0) "1,1,1") false false)
            (Utilities|FlowControl|Delay 1.0)
            (Transformation|AttachComponentToComponent Attach_To "None" "SnapToTarget" "SnapToTarget" "KeepWorld" false)
            (Variables|Default|SetIsAtach? true)
            (Timeline|Timeline_0 SetNewTime)))))))

(fn ConstructionScript)