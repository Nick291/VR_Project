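; BP_Pacient_01 is a patient actor that accepts a mask item brought into its Capsule trigger.
; An overlapping actor whose root component is tagged Maska_01 receives AttachingMessage with the patient's Mask component as the target.
; The patient then clears the first-person character's HeldObject, hides its Mask component, flags IsMaskAttach and reveals the SMBalloon component.
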(event OnComponentBeginOverlap(Capsule)
  (params (OverlappedComponent :type Primitive%20Component%20Object%20Reference) (OtherActor :type Actor%20Object%20Reference) (OtherComp :type Primitive%20Component%20Object%20Reference) (OtherBodyIndex :type Integer) (bFromSweep :type Boolean) (SweepResult :type Hit%20Result%20Structure%20%28by%20ref%29))
  (if (Components|ComponentHasTag (Variables|/Script/Engine.Actor|GetRootComponent OtherActor) "Maska_01")
    (Class|BPIActions|Attaching(Message) OtherActor (Variables|Default|GetMask))
    (bind _asfirst_person_character (Utilities|Casting|CastToFirstPersonCharacter (Game|GetPlayerCharacter 0)))
    (Variables|/Game/FirstPersonBP/Blueprints/FirstPersonCharacter.FirstPersonCharacter_C|SetHeldObject _asfirst_person_character 0)
    (Rendering|SetVisibility (Variables|Default|GetMask) false false)
    (Variables|Default|SetIsMaskAttach? true)
    (Rendering|SetVisibility (Variables|Default|GetSM_Balloon) true false)))

(event OnComponentEndOverlap(Capsule)
  (params (OverlappedComponent :type Primitive%20Component%20Object%20Reference) (OtherActor :type Actor%20Object%20Reference) (OtherComp :type Primitive%20Component%20Object%20Reference) (OtherBodyIndex :type Integer)))

(event EventBeginPlay)

(event Collision|EventActorBeginOverlap
  (params (OtherActor :type Actor%20Object%20Reference)))

(event EventTick
  (params (DeltaSeconds :type Float%20%28single-precision%29)))

(fn ConstructionScript)